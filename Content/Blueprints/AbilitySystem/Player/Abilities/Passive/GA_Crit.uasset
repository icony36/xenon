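; GA_Crit is a passive player gameplay ability that applies attack damage with a chance to crit.
; On activation it waits for Event.Attack gameplay events and takes the target from each payload.
; A CritChance roll decides whether the level-based damage is multiplied by CritDamage.
; Both outcomes deal damage with a long hit reaction, and each event also prints a debug string.
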(event `self.K2_ActivateAbility`
  (bind _returnvalue (`BlueprintGameplayTagLibrary.MakeLiteralGameplayTag` (struct :`TagName` "HitReact.Long")))
  (bind (_asynctaskproxy _payload) (`AbilityTask_WaitGameplayEvent.WaitGameplayEvent` (struct :`TagName` "Event.Attack") null)
    (:`EventReceived`
      (set `self.Target` (`.Target` (break `GameplayEventData` _payload)))
      (`KismetSystemLibrary.PrintString` "Hello" true true (struct :`G` 0.66 :`B` 1.0 :`A` 1.0) 3.0 "1")
      (bind _returnvalue_2 (`XeAbilitySystemLibrary.GetIsChanceSuccess` (`self.CritChance`)))
      (if _returnvalue_2
        (`self.CauseDamage` (`self.Target`) (* (`self.GetDamageAtLevel` true) (`self.CritDamage`)) true _returnvalue)
        (else
          (`self.CauseDamage` (`self.Target`) (`self.GetDamageAtLevel` true) true _returnvalue))))))