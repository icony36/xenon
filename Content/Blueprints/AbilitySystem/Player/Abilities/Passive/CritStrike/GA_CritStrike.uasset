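; Passive crit strike gameplay ability that gives attacks a chance to deal multiplied damage.
; ApplyAttackModifier rolls against CritChance and, on success, scales incoming damage by CritRate and reports that it applied.
; On activation it waits for the CritStrike gameplay event, then prints the event magnitude and spawns a pooled BP_FloatingText at the target.
; The floating text is not given the damage value here.
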(event `self.K2_ActivateAbility`
  (bind (_asynctaskproxy _payload) (`AbilityTask_WaitGameplayEvent.WaitGameplayEvent` (struct :`TagName` "Ability.Skill.Passive.CritStrike") null)
    (:`EventReceived`
      (bind (_eventtag _instigator _target _optionalobject _optionalobject2 _contexthandle _instigatortags _targettags _eventmagnitude) (break `GameplayEventData` _payload))
      (`KismetSystemLibrary.PrintString` (`KismetStringLibrary.Conv_DoubleToString` _eventmagnitude) true true (struct :`R` 1.0 :`G` 0.065068 :`A` 1.0) 1.0)
      (`PoolSubsystem.SpawnFromPool` (subsystem `PoolSubsystem`) "/Game/Blueprints/UI/FloatingText/BP_FloatingText.BP_FloatingText_C" (`Actor.K2_GetActorLocation` _target) (`Actor.K2_GetActorRotation` _target)))))

(fn `ApplyAttackModifier`
  (params (InDamage :type "Float (single-precision) (by ref)"))
  (returns (OutDamage :type "Float (single-precision)") (ReturnValue :type Boolean))
  (bind _returnvalue (`XeAbilitySystemLibrary.GetIsChanceSuccess` (`self.CritChance`)))
  (if _returnvalue
    (return (* InDamage (`self.CritRate`)) true)))