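; Gameplay ability for the player's FireBolt, an active ability that casts a projectile.
; On activation it plays the first ability montage and waits once for the Event.Cast gameplay event.
; That event spawns the projectile at the montage entry's cast socket, then ends the ability after a delay.
; Montage completion, interruption or cancellation also ends it, and ending the ability leaves the montage playing.
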(event `self.K2_ActivateAbility`
  (bind (_montage _castsocket) (break `TaggedMontage` (`|GetArrayItem` (`self.AbilityMontages`))))
  (`KismetSystemLibrary.PrintString` "Activate Firebot")
  (set `self.AvatarActor` (`self.GetAvatarActorFromActorInfo`))
  (set `self.CastSocket` _castsocket)
  (`AbilityTask_PlayMontageAndWait.CreatePlayMontageAndWaitProxy` "None" _montage 1.0 "None" false
    (:`then`
      (`AbilityTask_WaitGameplayEvent.WaitGameplayEvent` (struct :`TagName` "Event.Cast") null true
        (:`EventReceived`
          (`self.SpawnProjectile` (`self.CastSocket`))
          (`KismetSystemLibrary.Delay` 5.0)
          (`self.K2_EndAbility`))))
    (:`OnCompleted`
      (`self.K2_EndAbility` :!label _label))
    (:`OnInterrupted`
      (goto _label))
    (:`OnCancelled`
      (goto _label))))