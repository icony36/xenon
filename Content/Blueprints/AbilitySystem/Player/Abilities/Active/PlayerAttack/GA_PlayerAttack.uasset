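; Player melee attack gameplay ability that runs a five-stage, hold-to-charge combo from one montage, auto-facing the nearest combat actor.
; Montage gameplay events drive it: Start jumps to the stage's End section upon input release, Cast deals radial frontal damage with hit effects, End finishes.
; A press after Cast chains to the next stage using the section cached against blending errors.
; An early release is cached to skip the next charge.
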(event `self.K2_ActivateAbility`
  ;[1 1 1] Initialize Variables
  (set `self.ShouldSkipCharge` false)
  ;[1 1 1] Set Ignore Actors
  (set `self.ActorsToIgnore` (`|MakeArray` (`self.GetAvatarActorFromActorInfo`)))
  ;[1 1 1] Rotate to Target and Play Montage
  (`self.RotateToNearestTarget`)
  (`AbilityTask_PlayMontageAndWait.CreatePlayMontageAndWaitProxy` "None" (`.Montage` (break `TaggedMontage` (`self.GetMontageToPlay` false))) 1.0 "None" false
    (:`then`
      ;[1 1 1] Event Start
      (`AbilityTask_WaitGameplayEvent.WaitGameplayEvent` (struct :`TagName` "Event.Start") null
        (:`then`
          ;[1 1 1] Event Cast
          (`AbilityTask_WaitGameplayEvent.WaitGameplayEvent` (struct :`TagName` "Event.Cast") null
            (:`then`
              ;[1 1 1] Event End
              (`AbilityTask_WaitGameplayEvent.WaitGameplayEvent` (struct :`TagName` "Event.End") null
                (:`EventReceived`
                  (`self.K2_EndAbility`))))
            (:`EventReceived`
              (set `self.CurrentSection` (`self.GetCurrentMontageSection`)) ; Cached current section here as it might be wrong during blending.
              (`self.SpawnHitbox`)
              (`AbilityTask_WaitInputPress.WaitInputPress` false
                (:`then`
                  (`AbilityTask_WaitInputRelease.WaitInputRelease` false
                    (:`OnRelease`
                      (set `self.ShouldSkipCharge` true) ; Cache input is already released.
                    )))
                (:`OnPress`
                  (set `self.ShouldSkipCharge` false) ; Cache input is NOT yet released.
                  (`self.StartCombo`))))))
        (:`EventReceived`
          (if (`self.ShouldSkipCharge`)
            (set `self.ShouldSkipCharge` false)
            (else
              (`AbilityTask_WaitInputRelease.WaitInputRelease` false
                (:`OnRelease`
                  _))))
          (`self.JumpToCorrespondEnd`))))
    (:`OnCompleted`
      (`self.K2_EndAbility` :!label _label))
    (:`OnInterrupted`
      (goto _label))
    (:`OnCancelled`
      (goto _label))))

(event `StartCombo`
  ;[1 1 1] Start Combo
  (`self.RotateToNearestTarget`)
  (`self.JumpToNextCombo`))

(event `RotateToNearestTarget`
  ;[1 1 1] Rotate to Face Nearest Target
  (`self.RotateToFaceNearestCombatActor` (`self.ActorsToIgnore`) false 1.0 (struct :`G` 1.0 :`B` 0.97714 :`A` 1.0)))

(event `SpawnHitbox`
  ;[1 1 1] Handle Cast
  (bind _outoverlappingactors (`XeAbilitySystemLibrary.GetLiveCombatActorsWithinRadius` self (`self.ActorsToIgnore`) (`self.GetCastAtFrontLocation`) (`self.CastRadius`)))
  (for _array_element _outoverlappingactors
    (`self.CauseDamage` _array_element (`self.GetDamageAtLevel` true) true (`BlueprintGameplayTagLibrary.MakeLiteralGameplayTag` (struct :`TagName` "HitReact.Normal")))
    (`NiagaraFunctionLibrary.SpawnSystemAtLocation` "/Game/Assets/_ThirdParty/sA_Megapack_v1/sA_StylizedAttacksPack/FX/NiagaraSystems/NS_BasicHit_2.NS_BasicHit_2" (`Actor.K2_GetActorLocation` _array_element))))

(fn `GetEndSectionName`
  (returns (SectionName :type Name))
  (switch `name` (`self.GetCurrentMontageSection`)
    (:`Default`
      _)
    (:`1Loop`
      _)
    (:`2Start`
      (return "2End"))
    (:`2Loop`
      (return "2End"))
    (:`3Start`
      (return "3End"))
    (:`3Loop`
      (return "3End"))
    (:`4Start`
      (return "4End"))
    (:`4Loop`
      (return "4End"))
    (:`5Start`
      (return "5End"))
    (:`5Loop`
      (return "5End")))
  (return "1End"))

(fn `GetNextSectionName`
  (returns (SectionName :type Name))
  (switch `name` (`self.CurrentSection`)
    (:`1End`
      (return "2Start"))
    (:`2End`
      (return "3Start"))
    (:`3End`
      (return "4Start"))
    (:`4End`
      (return "5Start"))))

(fn `JumpToCorrespondEnd`
  (`self.MontageJumpToSection` (`self.GetEndSectionName`)))

(fn `JumpToNextCombo`
  (`self.MontageJumpToSection` (`self.GetNextSectionName`)))