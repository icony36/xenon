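; GA_HitReact is a gameplay ability, triggered by a gameplay event, that plays a character's hit reaction.
; It applies GE_HitReact to the owner, asks the avatar for a montage matching the event's first target tag, and snaps its yaw to face the instigator before playing it.
; Montage completion, interruption, cancellation, an Event.End gameplay event or a missing montage removes the effect and ends the ability.
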(event `self.K2_ActivateAbilityFromEvent`
  (params (EventData :type "GameplayEventData Structure (by ref)"))
  (bind (_eventtag _instigator _target _optionalobject _optionalobject2 _contexthandle _instigatortags _targettags) (break `GameplayEventData` EventData))
  (bind _returnvalue (`self.BP_ApplyGameplayEffectToOwner` "/Game/Blueprints/AbilitySystem/Common/Abilities/HitReact/GE_HitReact.GE_HitReact_C"))
  (set `self.ActiveEffectHandle` _returnvalue)
  (set `self.Instigator` _instigator)
  (bind _returnvalue_2 (message `CombatInterface.GetHitReactMontage` (`self.GetAvatarActorFromActorInfo`) (`|GetArrayItem` (`BlueprintGameplayTagLibrary.BreakGameplayTagContainer` _targettags))))
  (`/Engine/EditorBlueprintResources/StandardMacros.IsValid` _returnvalue_2
    (:`Is Valid`
      (`self.RotateToInstigator`)
      (`AbilityTask_PlayMontageAndWait.CreatePlayMontageAndWaitProxy` "None" _returnvalue_2 1.0 "None" false
        (:`then`
          (`AbilityTask_WaitGameplayEvent.WaitGameplayEvent` (struct :`TagName` "Event.End") null
            (:`EventReceived`
              (`self.HandleEnd`))))
        (:`OnCompleted`
          (`self.HandleEnd` :!label _label))
        (:`OnInterrupted`
          (goto _label))
        (:`OnCancelled`
          (goto _label))))
    (:`Is Not Valid`
      (`self.HandleEnd`))))

(event `HandleEnd`
  (`self.BP_RemoveGameplayEffectFromOwnerWithHandle` (`self.ActiveEffectHandle`))
  (`self.K2_EndAbility`))

(fn `RotateToInstigator`
  (bind _returnvalue (`self.GetAvatarActorFromActorInfo`))
  (bind _instigator (`self.Instigator`)
    (:`then`
      (`Actor.K2_SetActorRotation` (`self.GetAvatarActorFromActorInfo`) (`KismetMathLibrary.MakeRotator` (.roll (`Actor.K2_GetActorRotation` _returnvalue)) (.pitch (`Actor.K2_GetActorRotation` _returnvalue)) (.yaw (`KismetMathLibrary.FindLookAtRotation` (`Actor.K2_GetActorLocation` _returnvalue) (`Actor.K2_GetActorLocation` _instigator)))) false))
    (:`else`)))