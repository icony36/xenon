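; Anim notify state that turns the player character in place while the notify window of an animation is active.
; Each tick, if the cached PlayerCharacter is valid, it adds horizontal move input times TurnSpeed to the actor's yaw and zeroes pitch and roll.
; The yaw step is not scaled by frame delta time, so turn rate depends on tick rate.
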(fn `Received_NotifyTick`
  (params (MeshComp :type "SkeletalMeshComponent Object Reference") (Animation :type "AnimSequenceBase Object Reference") (FrameDeltaTime :type "Float (single-precision)") (EventReference :type "AnimNotifyEventReference Structure (by ref)"))
  (returns (ReturnValue :type Boolean))
  (bind _playercharacter (`self.PlayerCharacter`)
    (:`then`
      (`Actor.K2_SetActorRotation` (`self.PlayerCharacter`) (`KismetMathLibrary.MakeRotator` 0.0 0.0 (+ (* (.x (`XePlayerCharacter.MoveInputValue` _playercharacter)) (`self.TurnSpeed`)) (.yaw (`Actor.K2_GetActorRotation` _playercharacter)))) false)
      (return false))
    (:`else`)))